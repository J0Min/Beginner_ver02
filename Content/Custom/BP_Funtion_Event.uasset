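; BP_Funtion_Event is a Blueprint that demonstrates custom events and functions with a simple health value.
; On BeginPlay it prints a message and calls the AddHealth custom event, which prints the result of IncreaseHealth.
; IncreaseHealth and DecreaseHealth return CurrentHealth plus or minus their input without storing it, so health never changes.
; DecreaseHealth is unused, Tick is empty, and a few stray nodes are disconnected.
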(event `self.ReceiveBeginPlay`
  (`KismetSystemLibrary.PrintString` "Call Custom")
  (`self.AddHealth`))

(event `self.ReceiveTick`
  (params (DeltaSeconds :type "Float (single-precision)")))

(event `EnhancedInput|/Game/ThirdPerson/Input/Actions/IA_Jump`
  (params (ActionValue :type Boolean) (ElapsedSeconds :type "Float (double-precision)") (TriggeredSeconds :type "Float (double-precision)") (InputAction :type "InputAction Object Reference" :default "/Game/ThirdPerson/Input/Actions/IA_Jump.IA_Jump")))

(event `AddHealth`
  (`KismetSystemLibrary.PrintString` "Custom Event Start")
  (bind _returnhealth (`self.Increase Health` 10.0))
  (`KismetSystemLibrary.PrintString` (`KismetStringLibrary.Conv_DoubleToString` _returnhealth)))

(fn `Decrease Health`
  (params (SubtractHealth :type "Float (double-precision)"))
  (returns (ReturnHealth :type "Float (double-precision)"))
  (return (- (`self.CurrentHealth`) SubtractHealth)))

(fn `Increase Health`
  (params (`Add Health` :type "Float (double-precision)"))
  (returns (ReturnHealth :type "Float (double-precision)"))
  (return (+ (`self.CurrentHealth`) `Add Health`)))

(fn `UserConstructionScript`)