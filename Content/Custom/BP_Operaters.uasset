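; BP_Operaters is a scratch Blueprint that demonstrates math, comparison and boolean operator nodes.
; On BeginPlay it prints three results on screen: an addition, a tolerance-based float equality check and a boolean AND.
; Korean comments note that type conversion works only for numbers and that nearly-equal comparison compensates for float precision differences.
; Many other operator nodes sit unconnected in the graph, and the construction script is empty.
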(event `self.ReceiveBeginPlay`
  (`KismetSystemLibrary.PrintString` (`KismetStringLibrary.Conv_DoubleToString` (+ (`self.A`) (`self.D`))) true true (struct :`G` 0.66 :`B` 1.0 :`A` 1.0) 60.0)
  (`KismetSystemLibrary.PrintString` (`KismetStringLibrary.Conv_BoolToString` (`KismetMathLibrary.NearlyEqual_FloatFloat` (`self.A_0`) (`self.B_0`) 1.0)) true true (struct :`G` 0.66 :`B` 1.0 :`A` 1.0) 60.0)
  (`KismetSystemLibrary.PrintString` (`KismetStringLibrary.Conv_BoolToString` (and (`self.E`) (`self.F`))) true true (struct :`G` 0.66 :`B` 1.0 :`A` 1.0) 60.0))

(fn `UserConstructionScript`)