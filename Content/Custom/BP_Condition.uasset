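; BP_Condition is a practice Blueprint that demonstrates conditional flow nodes by printing results on BeginPlay.
; A Sequence runs a Branch on a Boolean, a Switch on an integer Selection, a Switch on a CurrentDirection enum that groups forward/backward and left/right, and a SelectInt driven by the same Boolean.
; Several unconnected Branch, Switch and Select nodes remain in the graph.
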(event `self.ReceiveBeginPlay`
  (`|ExecutionSequence`
    (:`then_0`
      (if (`self.Boolean`)
        (`KismetSystemLibrary.PrintString` "True Hello" true true (struct :`R` 0.708333 :`G` 1.0 :`B` 0.416667 :`A` 1.0) 60.0)
        (else
          (`KismetSystemLibrary.PrintString` "False Bye" true true (struct :`R` 1.0 :`G` 0.822969 :`B` 0.489158 :`A` 1.0) 60.0))))
    (:`then_1`
      (switch `int` (`self.Selection`)
        (:`Default`
          (`KismetSystemLibrary.PrintString` "Default" true true (struct :`R` 0.708333 :`G` 1.0 :`B` 0.416667 :`A` 1.0) 60.0))
        (:`0`
          (`KismetSystemLibrary.PrintString` "0" true true (struct :`R` 0.708333 :`G` 1.0 :`B` 0.416667 :`A` 1.0) 60.0))
        (:`1`
          (`KismetSystemLibrary.PrintString` "1" true true (struct :`R` 0.708333 :`G` 1.0 :`B` 0.416667 :`A` 1.0) 60.0))
        (:`2`
          (`KismetSystemLibrary.PrintString` "2" true true (struct :`R` 0.708333 :`G` 1.0 :`B` 0.416667 :`A` 1.0) 60.0))))
    (:`then_2`
      (switch `/Game/Custom/E_Condtion_Example` (`self.CurrentDirection`)
        (:`NewEnumerator0`
          (`KismetSystemLibrary.PrintString` "앞뒤" true true (struct :`R` 0.708333 :`G` 1.0 :`B` 0.416667 :`A` 1.0) 60.0 :!label _label))
        (:`NewEnumerator1`
          (goto _label))
        (:`NewEnumerator2`
          (`KismetSystemLibrary.PrintString` "좌우" true true (struct :`R` 0.708333 :`G` 1.0 :`B` 0.416667 :`A` 1.0) 60.0 :!label _label_2))
        (:`NewEnumerator3`
          (goto _label_2))))
    (:`then_3`
      (`KismetSystemLibrary.PrintString` (`KismetStringLibrary.Conv_IntToString` (`KismetMathLibrary.SelectInt` 10 20 (`self.Boolean`))) true true (struct :`R` 1.0 :`G` 0.822969 :`B` 0.489158 :`A` 1.0) 60.0))))

(fn `UserConstructionScript`)