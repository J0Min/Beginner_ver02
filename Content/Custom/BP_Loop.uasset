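; BP_Loop is a Blueprint that demonstrates the loop types by printing values to the screen at BeginPlay.
; A Sequence runs a For Loop, a For Loop with Break, a For Each over TestForEach, and a While Loop counting Current up to Max, in that order.
; Each loop prints in its own color.
; Extra unconnected loop nodes in the graph never run.
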(event `self.ReceiveBeginPlay`
  (bind _current (`self.Current`))
  (`|ExecutionSequence`
    (:`then_0`
      (for _index (range 5)
        (`KismetSystemLibrary.PrintString` (`KismetStringLibrary.Conv_IntToString` _index) true true (struct :`R` 0.661841 :`G` 0.184235 :`B` 1.0 :`A` 1.0) 10.0)))
    (:`then_1`
      (for _index_2 (range 101)
        (`KismetSystemLibrary.PrintString` (`KismetStringLibrary.Conv_IntToString` _index_2) true true (struct :`G` 0.101157 :`B` 1.0 :`A` 1.0) 10.0)
        (if (>= _index_2 5)
          (break))))
    (:`then_2`
      (for _array_element (`self.test_For_each`)
        (`KismetSystemLibrary.PrintString` _array_element true true (struct :`R` 0.734426 :`G` 1.0 :`B` 0.886866 :`A` 1.0) 10.0)))
    (:`then_3`
      (while (< (`self.Current`) (`self.Max`))
        (`KismetSystemLibrary.PrintString` (`KismetStringLibrary.Conv_DoubleToString` _current) true true (struct :`R` 0.913544 :`G` 1.0 :`B` 0.502502 :`A` 1.0) 10.0)
        (`/Engine/EditorBlueprintResources/StandardMacros.IncrementFloat` _current)))))

(fn `UserConstructionScript`)