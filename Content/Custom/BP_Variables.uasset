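; BP_Variables is a test Blueprint that demonstrates setting and printing basic variables: character name, death flag, health and item count.
; On BeginPlay it prints a formatted summary of the four values, assigns new ones, then prints the summary again to show the change.
; Separate print and reset chains are left unconnected and never run.
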(event `self.ReceiveBeginPlay`
  (bind _returnvalue (`KismetTextLibrary.Conv_TextToString` (`|FormatText` "Character Name : {Name}, isDead : {isDead}, Current Health : {Health}, Item Count : {ItemCount}" (`self.Name`) (`self.isDead`) (`self.Health`) (`self.ItemCount`))))
  (`KismetSystemLibrary.PrintString` _returnvalue true true (struct :`G` 0.66 :`B` 1.0 :`A` 1.0) 300.0)
  (set `self.isDead` false)
  (set `self.Health` 157.4)
  (set `self.ItemCount` -10)
  (set `self.Name` "Free")
  (`KismetSystemLibrary.PrintString` _returnvalue true true (struct :`G` 0.66 :`B` 1.0 :`A` 1.0) 300.0))

(fn `UserConstructionScript`)